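; Bee character that endlessly forages between flowers and hives, starting with a flower trip on BeginPlay.
; SeekFlower and SeekHive each pick a random actor derived from the flower or hive base class and travel there with AIMoveTo.
; When a move finishes, a short delay precedes the opposite seek event.
; Hive arrivals also call BeeDeposit on the main widgets, found by class.
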(event Custom|SeekFlower
  ;[0 0 0] Once called get array of actors from parent Flower, randomize and then move to and wait then seek hive
  (bind _outactors (Actor|GetAllActorsOfClass "/Game/Blueprints/Flowers/BP_FlowersBase.BP_FlowersBase_C"))
  (bind _output_get (Variables|Default|SetTargetFlower (Utilities|Array|Get(acopy) _outactors (Math|Random|RandomIntegerinRange 0 (Utilities|Array|LastIndex _outactors)))))
  (AI|AIMoveTo (AI|GetAIController self) "0, 0, 0" _output_get 1e+01 "Default" "Default" true true
    (:OnMoveFinished
      (Development|PrintString "at flower")
      (Utilities|FlowControl|Delay 0.6)
      (CallFunction|SeekHive))))

(event Custom|SeekHive
  ;[0 0 0] Once called get array of actors from parent Hive, randomize and then move to and wait then seek flower
  (bind _outactors (Actor|GetAllActorsOfClass "/Game/Blueprints/Hives/BP_HiveBase.BP_HiveBase_C"))
  (bind _output_get (Variables|Default|SetTargetHive (Utilities|Array|Get(acopy) _outactors (Math|Random|RandomIntegerinRange 0 (Utilities|Array|LastIndex _outactors)))))
  (AI|AIMoveTo (AI|GetAIController self) "0, 0, 0" _output_get 1e+02 "Default" "Default" true true
    (:OnMoveFinished
      (bind _foundwidgets (Widget|GetAllWidgetsOfClass "/Game/Blueprints/BP_MainWidget.BP_MainWidget_C" false))
      (Default|BeeDeposit _foundwidgets)
      (Development|PrintString "at hive")
      (Utilities|FlowControl|Delay 0.4)
      (CallFunction|SeekFlower))))

(event EventBeginPlay
  ;[0 0 0] Once spawned seek flower
  (CallFunction|SeekFlower))

(fn ConstructionScript)